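; BP_SurvivalCharacter is the survival character Blueprint, handling keyboard input for item granting and hotbar use.
; R and T each look up a hardcoded DT_Items row and send it to the Inventory and Hotbar respectively through ServerAddItem.
; Number keys 1–9 pass a zero-based slot index to ServerHotbarInput, which is defined outside these graphs.
; BeginPlay, overlap, Tick and the construction script are empty.
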(event EventBeginPlay)

(event Collision|EventActorBeginOverlap
  (params (OtherActor :type Actor%20Object%20Reference)))

(event EventTick
  (params (DeltaSeconds :type Float%20%28single-precision%29)))

(event Input|KeyboardEvents|1
  (params (Key :type Key%20Structure :default "None"))
  (:Pressed
    (Class|SurvivalCharacter|ServerHotbarInput)))

(event Input|KeyboardEvents|2
  (params (Key :type Key%20Structure :default "None"))
  (:Pressed
    (Class|SurvivalCharacter|ServerHotbarInput 1)))

(event Input|KeyboardEvents|R
  (params (Key :type Key%20Structure :default "None"))
  (:Pressed
    (bind _returnvalue (Utilities|GetDataTableRow "/Game/Blueprints/DataTables/DT_Items.DT_Items" "2")
      (:then
        (Class|ItemContainer|ServerAddItem (Variables|Default|GetInventory) _returnvalue)))))

(event Input|KeyboardEvents|3
  (params (Key :type Key%20Structure :default "None"))
  (:Pressed
    (Class|SurvivalCharacter|ServerHotbarInput 2)))

(event Input|KeyboardEvents|4
  (params (Key :type Key%20Structure :default "None"))
  (:Pressed
    (Class|SurvivalCharacter|ServerHotbarInput 3)))

(event Input|KeyboardEvents|5
  (params (Key :type Key%20Structure :default "None"))
  (:Pressed
    (Class|SurvivalCharacter|ServerHotbarInput 4)))

(event Input|KeyboardEvents|6
  (params (Key :type Key%20Structure :default "None"))
  (:Pressed
    (Class|SurvivalCharacter|ServerHotbarInput 5)))

(event Input|KeyboardEvents|7
  (params (Key :type Key%20Structure :default "None"))
  (:Pressed
    (Class|SurvivalCharacter|ServerHotbarInput 6)))

(event Input|KeyboardEvents|8
  (params (Key :type Key%20Structure :default "None"))
  (:Pressed
    (Class|SurvivalCharacter|ServerHotbarInput 7)))

(event Input|KeyboardEvents|9
  (params (Key :type Key%20Structure :default "None"))
  (:Pressed
    (Class|SurvivalCharacter|ServerHotbarInput 8)))

(event Input|KeyboardEvents|T
  (params (Key :type Key%20Structure :default "None"))
  (:Pressed
    (bind _returnvalue (Utilities|GetDataTableRow "/Game/Blueprints/DataTables/DT_Items.DT_Items" "3")
      (:then
        (Class|ItemContainer|ServerAddItem (Variables|Default|GetHotbar) _returnvalue)))))

(fn ConstructionScript)