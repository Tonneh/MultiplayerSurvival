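; BP_PalmDestructableMaster is a destructible palm tree base that dissolves out of view shortly after it begins play.
; After the parent BeginPlay and a short delay, it creates dynamic material instances for the static mesh's bark and leaf slots.
; The FadeAway timeline drives the Dissolve parameter on all of them, then hides the mesh when finished without destroying the actor.
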(event EventBeginPlay
  (|CallParentFunction)
  (Utilities|FlowControl|Delay 5.0)
  (bind _returnvalue (Rendering|Material|CreateDynamicMaterialInstance (Variables|Default|GetStaticMesh) 0 "/Game/Assets/PalmTrees/Materials/M_Palm01.M_Palm01" "None" :!class /Script/Engine.PrimitiveComponent))
  (Variables|Default|SetMat0 _returnvalue)
  (bind _returnvalue_2 (Rendering|Material|CreateDynamicMaterialInstance (Variables|Default|GetStaticMesh) 1 "/Game/Assets/PalmTrees/Materials/M_Palm02.M_Palm02" "None" :!class /Script/Engine.PrimitiveComponent))
  (Variables|Default|SetMat1 _returnvalue_2)
  (bind _returnvalue_3 (Rendering|Material|CreateDynamicMaterialInstance (Variables|Default|GetStaticMesh) 2 "/Game/Assets/PalmTrees/Materials/M_Palm03.M_Palm03" "None" :!class /Script/Engine.PrimitiveComponent))
  (Variables|Default|SetMat2 _returnvalue_3)
  (bind _returnvalue_4 (Rendering|Material|CreateDynamicMaterialInstance (Variables|Default|GetStaticMesh) 3 "/Game/Assets/PalmTrees/Materials/M_Palm03.M_Palm03" "None" :!class /Script/Engine.PrimitiveComponent))
  (Variables|Default|SetMat3 _returnvalue_4)
  (bind _returnvalue_5 (Rendering|Material|CreateDynamicMaterialInstance (Variables|Default|GetStaticMesh) 4 "/Game/Assets/PalmTrees/Materials/M_PalmLeaf_Inst.M_PalmLeaf_Inst" "None" :!class /Script/Engine.PrimitiveComponent))
  (Variables|Default|SetMat4 _returnvalue_5)
  (bind _returnvalue_6 (Rendering|Material|CreateDynamicMaterialInstance (Variables|Default|GetStaticMesh) 5 "/Game/Assets/PalmTrees/Materials/M_Palm04.M_Palm04" "None" :!class /Script/Engine.PrimitiveComponent))
  (Variables|Default|SetMat5 _returnvalue_6)
  (bind _newtrack_0 (Timeline|FadeAway PlayFromStart)
    (:Update
      (Rendering|Material|SetScalarParameterValue (Variables|Default|GetMat0) "Dissolve" _newtrack_0 :!class /Script/Engine.MaterialInstanceDynamic))
    (:Finished
      (Rendering|SetVisibility (Variables|Default|GetStaticMesh) false false))))

(fn ConstructionScript
  (|CallParentFunction))