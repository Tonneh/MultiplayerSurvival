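; Player controller for the survival game that relays inventory, crafting, harvest and player stat events to the main HUD widget.
; It caches the WBP_MainWidget on BeginPlay, and several paths lazily re-fetch it when the reference is invalid.
; Slot updates resolve the grid by container type, with only inventory and hotbar wired, and adding an item also refreshes crafting requirements.
; Other events drive the crafting bar, stat bars, and starving and dehydration notifications.
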(event EventBeginPlay
  (bind _aswbp_main_widget (Utilities|Casting|CastToWBP_MainWidget (Class|SurvivalPlayerController|GetMainWidget)))
  (Variables|Default|SetMainWidgetRef _aswbp_main_widget))

(event EventTick
  (params (DeltaSeconds :type Float%20%28single-precision%29)))

(event EventShoworHideDehydration
  (params (ShowOrHide :type Boolean))
  (bind _mainwidgetref (Variables|Default|GetMainWidgetRef))
  ;[1 1 1] Show or Hide Starving/Dehydration
  (CallFunction|InitMainWidgetRef)
  (Utilities|IsValid _mainwidgetref
    (:Is%20Valid
      (if ShowOrHide
        (Default|ShowDehydratedNotification _mainwidgetref)
        (else
          (Default|RemoveDehydratedNotification _mainwidgetref))))))

(event EventBPShowProgressBar
  ;[1 1 1] Update Crafting Progress Bar
  (Default|ShowCraftingBar (Variables|Default|GetMainWidgetRef)))

(event EventSetInventoryVis
  (params (Visibility :type Boolean))
  ;[1 1 1] Toggle Inventory
  (bind _mainwidgetref (Variables|Default|GetMainWidgetRef)
    (:then
      _)
    (:else
      (bind _aswbp_main_widget (Utilities|Casting|CastToWBP_MainWidget (Class|SurvivalPlayerController|GetMainWidget)))
      (bind _output_get (Variables|Default|SetMainWidgetRef _aswbp_main_widget))))
  (Default|SetInventoryVis _mainwidgetref Visibility))

(event EventBPUpdateStatBar
  (params (Stat :type EPlayerStats%20Enum :default "Health") (Curr :type Float%20%28single-precision%29) (Max :type Float%20%28single-precision%29))
  (bind _mainwidgetref (Variables|Default|GetMainWidgetRef))
  ;[1 1 1] Update Stat bar
  (CallFunction|InitMainWidgetRef)
  (Utilities|IsValid _mainwidgetref
    (:Is%20Valid
      (Default|UpdateBar (Variables|/Game/Blueprints/Widgets/WBP_MainWidget.WBP_MainWidget_C|GetWBP_PlayerStatsWindow _mainwidgetref) Stat Curr Max))))

(event EventBPUpdateCraftStatus
  (params (CanCraft :type Boolean))
  (bind _mainwidgetref (Variables|Default|GetMainWidgetRef))
  (bind _wbp_inventory (Variables|/Game/Blueprints/Widgets/WBP_MainWidget.WBP_MainWidget_C|GetWBP_Inventory _mainwidgetref))
  (bind _wbp_craftingwindow (Variables|/Game/Blueprints/Widgets/InventoryWidget/WBP_Inventory.WBP_Inventory_C|GetWBP_CraftingWindow _wbp_inventory))
  ;[1 1 1] Update Craft Status
  (Utilities|IsValid _wbp_craftingwindow
    (:Is%20Valid
      (Default|UpdateCraftingStatus _wbp_craftingwindow CanCraft))))

(event EventShoworHideStarving
  (params (ShowOrHide :type Boolean))
  (bind _mainwidgetref (Variables|Default|GetMainWidgetRef))
  ;[1 1 1] Show or Hide Starving/Dehydration
  (CallFunction|InitMainWidgetRef)
  (Utilities|IsValid _mainwidgetref
    (:Is%20Valid
      (if ShowOrHide
        (Default|ShowStarvingNotification _mainwidgetref)
        (else
          (Default|RemoveStarvingNotification _mainwidgetref))))))

(event EventBPShowHarvestedItemWidget
  (params (ResourceImage :type Texture%202D%20Object%20Reference) (ResourceQuantity :type Integer) (ResourceName :type Name :default "None"))
  ;[1 1 1] Update Item Collected
  (Default|ShowItemCollected (Variables|Default|GetMainWidgetRef) ResourceImage ResourceQuantity (Utilities|Text|ToText(Name) ResourceName)))

(event EventBPResetItemSlot
  (params (Container :type EContainerType%20Enum :default "EContainerType_PlayerInventory") (Index :type Integer))
  ;[1 1 1] Updating inventory UI for when Removing items
  (bind _widget (CallFunction|GetInventoryWidget Container Index))
  (Utilities|IsValid _widget
    (:Is%20Valid
      (Default|ResetSlot _widget))))

(event EventBPUpdateItemSlot
  (params (Container :type EContainerType%20Enum :default "EContainerType_PlayerInventory") (Index :type Integer) (ItemInfo :type Item%20Info%20Structure))
  ;[1 1 1] Updating inventory UI for when adding items
  (bind _widget (CallFunction|GetInventoryWidget Container Index))
  (Utilities|IsValid _widget
    (:Is%20Valid
      (Default|UpdateSlot _widget ItemInfo)
      (Default|ShowItemRequirements (Variables|/Game/Blueprints/Widgets/InventoryWidget/WBP_Inventory.WBP_Inventory_C|GetWBP_CraftingWindow (Variables|/Game/Blueprints/Widgets/WBP_MainWidget.WBP_MainWidget_C|GetWBP_Inventory (Variables|Default|GetMainWidgetRef))) Index))))

(fn ConstructionScript)

(fn GetInventoryWidget
  (params (Container :type EContainerType%20Enum :default "EContainerType_PlayerInventory") (SlotIndex :type Integer))
  (Variables|Default|GetMainWidgetRef
    (:then
      _)
    (:else
      (bind _aswbp_main_widget (Utilities|Casting|CastToWBP_MainWidget (Class|SurvivalPlayerController|GetMainWidget)))
      (Variables|Default|SetMainWidgetRef _aswbp_main_widget)))
  (return (Utilities|Array|Get(acopy) (Variables|/Game/Blueprints/Widgets/InventoryWidget/WBP_ItemContainerGrid.WBP_ItemContainerGrid_C|GetSlots (Utilities|Select :Index Container :EContainerType_PlayerInventory (Variables|/Game/Blueprints/Widgets/InventoryWidget/WBP_Inventory.WBP_Inventory_C|GetWBP_ItemContainerGrid (Variables|/Game/Blueprints/Widgets/WBP_MainWidget.WBP_MainWidget_C|GetWBP_Inventory (Variables|Default|GetMainWidgetRef))) :EContainerType_PlayerHotbar (Variables|/Game/Blueprints/Widgets/InventoryWidget/WBP_Hotbar.WBP_Hotbar_C|GetWBP_ItemContainerGrid (Variables|/Game/Blueprints/Widgets/WBP_MainWidget.WBP_MainWidget_C|GetWBP_Hotbar (Variables|Default|GetMainWidgetRef))) :EContainerType_PlayerStorage 0 :EContainerType_PlayerArmor 0)) SlotIndex)))

(fn InitMainWidgetRef
  (Variables|Default|GetMainWidgetRef
    (:then)
    (:else
      (bind _aswbp_main_widget (Utilities|Casting|CastToWBP_MainWidget (Class|SurvivalPlayerController|GetMainWidget)))
      (Variables|Default|SetMainWidgetRef _aswbp_main_widget))))